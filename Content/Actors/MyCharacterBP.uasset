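; MyCharacterBP is a character Blueprint that uses the Gameplay Ability System to grant and trigger abilities.
; On BeginPlay it passes each entry in AbilityClasses to AquireAbility.
; Two input actions activate the first and second classes by array index through the ASC, with remote activation allowed.
; Tick prints the character's name and current MyAttributeValue on screen as a debug readout.
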(event `InputAction|ActivateAbility1`
  (params (Key :type "Key Structure"))
  ;[1 1 1] Ability control
  (:`Pressed`
    (`AbilitySystemComponent.TryActivateAbilityByClass` (`self.ASC`) (`|GetArrayItem` (`self.AbilityClasses`)) true)))

(event `InputAction|ActivateAbility2`
  (params (Key :type "Key Structure"))
  ;[1 1 1] Ability control
  (:`Pressed`
    (`AbilitySystemComponent.TryActivateAbilityByClass` (`self.ASC`) (`|GetArrayItem` (`self.AbilityClasses`) 1) true)))

(event `self.ReceiveBeginPlay`
  ;[1 1 1] Ability control
  (for _array_element (`self.AbilityClasses`)
    (`self.AquireAbility` _array_element)))

(event `self.ReceiveTick`
  (params (DeltaSeconds :type "Float (single-precision)"))
  ;[1 1 1] Print current MyAttributeValue
  (`KismetSystemLibrary.PrintString` (`KismetStringLibrary.Concat_StrStr` (`KismetSystemLibrary.GetDisplayName` self) "    " (`KismetTextLibrary.Conv_TextToString` (`KismetTextLibrary.Conv_DoubleToText` (`.ReturnValue` (`AbilitySystemBlueprintLibrary.GetFloatAttributeFromAbilitySystemComponent` (`self.ASC`) (struct :`Attribute` "/Script/ue4_gas_prediction.MyAttributeSet:MyAttribute"))) "HalfToEven" false true 1 324 0 0))) true false (struct :`G` 0.66 :`B` 1.0 :`A` 1.0) 0.0))

(fn `UserConstructionScript`)